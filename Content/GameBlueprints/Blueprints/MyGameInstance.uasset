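; Game instance Blueprint that opens the multiplayer menus and handles hosting and joining of online sessions.
; Menu events lazily create and cache the SearchGames and HostGame widgets, then add them to the viewport.
; LaunchLobby stores the server name, creates a Steam or LAN session and opens TestMap as a listen server.
; JoinServer joins a given search result; both session calls print on failure.
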(event `SearchGameMenu`
  (`/Engine/EditorBlueprintResources/StandardMacros.IsValid` (`self.ServerBrowser`)
    (:`Is Valid`
      _)
    (:`Is Not Valid`
      (bind _returnvalue (`|CreateWidget` "/Game/GameBlueprints/Blueprints/SearchGames.SearchGames_C" (`GameplayStatics.GetPlayerController` 0)))
      (bind _output_get (set `self.ServerBrowser` _returnvalue))))
  (`UserWidget.AddToViewport` _output_get 0))

(event `HostGameMenu`
  (`/Engine/EditorBlueprintResources/StandardMacros.IsValid` (`self.HostGame`)
    (:`Is Valid`
      _)
    (:`Is Not Valid`
      (bind _returnvalue (`|CreateWidget` "/Game/GameBlueprints/Blueprints/HostGame.HostGame_C" (`GameplayStatics.GetPlayerController` 0)))
      (bind _output_get (set `self.HostGame` _returnvalue))))
  (`UserWidget.AddToViewport` _output_get 0))

(event `LaunchLobby`
  (params (UseSteam :type Boolean) (ServerName :type Text))
  (set `self.ServerName` ServerName)
  (`CreateSessionCallbackProxy.CreateSession` (`GameplayStatics.GetPlayerController` 0) 20 (not UseSteam)
    (:`OnSuccess`
      (`GameplayStatics.OpenLevel` "TestMap" true "listen"))
    (:`OnFailure`
      (`KismetSystemLibrary.PrintString` "Failed to open level "))))

(event `JoinServer`
  (params (Session :type "BlueprintSessionResult Structure"))
  (`JoinSessionCallbackProxy.JoinSession` (`GameplayStatics.GetPlayerController` 0) Session
    (:`OnFailure`
      (`KismetSystemLibrary.PrintString` "Couldnt join session."))))